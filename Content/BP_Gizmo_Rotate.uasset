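; Rotation gizmo that turns the player's active selection around world X, Y or Z with mouse movement.
; Clicking an axis mesh sets the selected axis from its tag; Tick applies rotation, gated by modifier-key, movement and facing checks.
; X and Y blend vertical and horizontal mouse deltas by axis orientation; Z uses horizontal only.
; Tick also snaps the parent actor to the selection, scales it by player distance and keeps the gizmo world-aligned.
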(event EventTick
  (params (DeltaSeconds :type Float%20%28single-precision%29))
  (Utilities|FlowControl|Sequence
    (:then_0
      (CallFunction|FRotateTarget))
    (:then_1
      (CallFunction|FGizmoSize))))

(event EventBeginPlay)

(event OnClicked(Y_Mesh)
  (params (TouchedComponent :type Primitive%20Component%20Object%20Reference) (ButtonPressed :type Key%20Structure))
  (Variables|Default|SetSelected_Axis (Utilities|Array|Get(acopy) (Variables|/Script/Engine.ActorComponent|GetComponentTags TouchedComponent))))

(event OnClicked(Z_Mesh)
  (params (TouchedComponent :type Primitive%20Component%20Object%20Reference) (ButtonPressed :type Key%20Structure))
  (Variables|Default|SetSelected_Axis (Utilities|Array|Get(acopy) (Variables|/Script/Engine.ActorComponent|GetComponentTags TouchedComponent))))

(event OnClicked(X_Mesh)
  (params (TouchedComponent :type Primitive%20Component%20Object%20Reference) (ButtonPressed :type Key%20Structure))
  (Variables|Default|SetSelected_Axis (Utilities|Array|Get(acopy) (Variables|/Script/Engine.ActorComponent|GetComponentTags TouchedComponent))))

(fn ConstructionScript)

(fn FRotateTarget
  (bind _defaultsceneroot (Variables|Default|GetDefaultSceneRoot))
  (Utilities|IsValid 0
    (:Is%20Valid
      (Utilities|IsValid 0
        (:Is%20Valid
          (if (not (Utilities|ForbiddenKeys))
            (if (Utilities|DetectMovement)
              (if (> (Math|Vector|DotProduct (Math|Vector|GetForwardVector _defaultsceneroot) (Math|Vector|Normalize (- (Transformation|GetWorldLocation _defaultsceneroot) (Transformation|GetWorldLocation _defaultsceneroot)))) 0.5)
                (switch name (Variables|Default|GetSelected_Axis)
                  (:X_Mesh
                    (CallFunction|FRotateX))
                  (:Y_Mesh
                    (CallFunction|FRotateY))
                  (:Z_Mesh
                    (CallFunction|FRotateZ)))
                (return)))))))))

(fn FGizmoSize
  (bind _ref_player (Variables|Referances|GetREF_Player))
  (bind _defaultsceneroot (Variables|Default|GetDefaultSceneRoot))
  (bind _returnvalue (Transformation|GetWorldLocation _defaultsceneroot))
  (bind _capsulecomponent (Variables|/Script/Engine.Character|GetCapsuleComponent _ref_player))
  (bind _returnvalue_2 (Transformation|GetWorldLocation _capsulecomponent))
  (bind _returnvalue_3 (Math|Vector|Distance(Vector) _returnvalue_2 _returnvalue))
  (bind _returnvalue_4 (/ _returnvalue_3 1.15e+03))
  (Transformation|SetWorldTransform (Variables|/Script/Engine.Actor|GetRootComponent (Actor|GetParentActor self)) (Math|Transform|MakeTransform (.location (Transformation|GetWorldTransform (Variables|Default|GetActive_Selection (.REF_Player (Variables|Referances|GetREF_Player))))) "0, 0, 0" (Math|Vector|MakeVector _returnvalue_4 _returnvalue_4 _returnvalue_4)) false false)
  (Transformation|SetWorldRotation (Variables|Default|GetDefaultSceneRoot) "0, 0, 0" false false)
  (return))

(fn FRotateY
  (bind _returnvalue (Game|GetPlayerController 0))
  (bind (_deltax _deltay) (Class|PlayerController|GetInputMouseDelta _returnvalue))
  (LocalVariables|SetAxis_Forward (Math|Vector|GetRightVector (Variables|Default|GetY_Mesh)))
  (LocalVariables|SetNormal_Vector (Utilities|HorizontalNormal (Variables|Default|GetY_Mesh)))
  (Transformation|AddWorldRotation (Variables|Default|GetActive_Selection (.REF_Player (Variables|Referances|GetREF_Player))) (Math|Rotator|MakeRotator 0.0 (Math|Float|Lerp (* _deltay (select (>= (Math|Float|Absolute(Float) (.z (LocalVariables|GetAxis_Forward))) 0.75) (select (>= (.z (LocalVariables|GetAxis_Forward)) 0.0) -5.0 5.0) (select (> (Math|Vector|DotProduct (LocalVariables|GetAxis_Forward) (LocalVariables|GetNormal_Vector)) 0.0) -5.0 5.0))) (* (select (> (.z (Math|Vector|CrossProduct (LocalVariables|GetAxis_Forward) (LocalVariables|GetNormal_Vector))) 0.0) 5.0 -5.0) _deltax) (Math|Float|Clamp(Float) (Math|Float|Absolute(Float) (.z (Math|Vector|CrossProduct (LocalVariables|GetAxis_Forward) (LocalVariables|GetNormal_Vector)))))) 0.0) false false)
  (return))

(fn FRotateX
  (bind _returnvalue (Game|GetPlayerController 0))
  (bind (_deltax _deltay) (Class|PlayerController|GetInputMouseDelta _returnvalue))
  (LocalVariables|SetAxis_Forward (Math|Vector|GetRightVector (Variables|Default|GetX_Mesh)))
  (LocalVariables|SetNormal_Vector (Utilities|HorizontalNormal (Variables|Default|GetX_Mesh)))
  (Transformation|AddWorldRotation (Variables|Default|GetActive_Selection (.REF_Player (Variables|Referances|GetREF_Player))) (Math|Rotator|MakeRotator (Math|Float|Lerp (* _deltay (select (>= (Math|Float|Absolute(Float) (.z (LocalVariables|GetAxis_Forward))) 0.75) (select (>= (.z (LocalVariables|GetAxis_Forward)) 0.0) 5.0 -5.0) (select (> (Math|Vector|DotProduct (LocalVariables|GetAxis_Forward) (LocalVariables|GetNormal_Vector)) 0.0) -5.0 5.0))) (* (select (> (.z (Math|Vector|CrossProduct (LocalVariables|GetAxis_Forward) (LocalVariables|GetNormal_Vector))) 0.0) 5.0 -5.0) _deltax) (Math|Float|Clamp(Float) (Math|Float|Absolute(Float) (.z (Math|Vector|CrossProduct (LocalVariables|GetAxis_Forward) (LocalVariables|GetNormal_Vector)))))) 0.0 0.0) false false)
  (return))

(fn FRotateZ
  (Transformation|AddWorldRotation (Variables|Default|GetActive_Selection (.REF_Player (Variables|Referances|GetREF_Player))) (Math|Rotator|MakeRotator 0.0 0.0 (* -5.0 (.DeltaX (Class|PlayerController|GetInputMouseDelta (Game|GetPlayerController 0))))) false false)
  (return))