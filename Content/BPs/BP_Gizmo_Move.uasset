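; BP_Gizmo_Move is a move gizmo with clickable mesh handles for the X, Y and Z axes plus a combined XYZ handle.
; Clicking a handle records its axis in AxisEnum and stores the clicked component in AxisComponent.
; The graphs shown only capture this selection and contain no movement logic; the construction script is empty.
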(event OnClicked(SM_Axis_X)
  (params (TouchedComponent :type Primitive%20Component%20Object%20Reference) (ButtonPressed :type Key%20Structure :default "None"))
  (Variables|Default|SetAxisEnum "X_Axis")
  (Variables|Default|SetAxisComponent TouchedComponent))

(event OnClicked(SM_Axis_Y)
  (params (TouchedComponent :type Primitive%20Component%20Object%20Reference) (ButtonPressed :type Key%20Structure :default "None"))
  (Variables|Default|SetAxisEnum "Y_Axis")
  (Variables|Default|SetAxisComponent TouchedComponent))

(event OnClicked(SM_Axis_Z)
  (params (TouchedComponent :type Primitive%20Component%20Object%20Reference) (ButtonPressed :type Key%20Structure :default "None"))
  (Variables|Default|SetAxisEnum "Z_Axis")
  (Variables|Default|SetAxisComponent TouchedComponent))

(event OnClicked(SM_Axis_XYZ)
  (params (TouchedComponent :type Primitive%20Component%20Object%20Reference) (ButtonPressed :type Key%20Structure :default "None"))
  (Variables|Default|SetAxisEnum "XYZ_Axis")
  (Variables|Default|SetAxisComponent TouchedComponent))

(fn ConstructionScript)