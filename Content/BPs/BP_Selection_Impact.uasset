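; BP_Selection_Impact is a short-lived effect actor that shows a growing sphere, apparently as feedback for a selection.
; On BeginPlay a timeline drives the sphere's relative scale, multiplied by the distance from the actor's root to the player character's capsule so the effect grows larger when farther away.
; The actor destroys itself when the timeline finishes.
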(event EventBeginPlay
  (bind _grow (Timeline|Timeline_Grow_Sphere Play)
    (:Update
      (Transformation|SetRelativeScale3D (Variables|Default|GetSphere) (Math|Conversions|ToVector(Float) (* _grow (/ (Math|Vector|Distance(Vector) (Transformation|GetWorldLocation (Variables|Default|GetDefaultSceneRoot)) (Transformation|GetWorldLocation (Variables|/Script/Engine.Character|GetCapsuleComponent (Game|GetPlayerCharacter 0)))) 7.5e+02)))))
    (:Finished
      (Actor|DestroyActor))))

(fn ConstructionScript)