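; Rotation gizmo, a child actor of GizmoBase, that lets the desktop player rotate the GizmoTarget with the mouse.
; Clicking an axis mesh stores its tag, and Tick turns mouse movement into world rotation on that axis, gated by modifier keys and camera facing.
; X and Y blend horizontal and vertical mouse deltas by camera-relative axis direction.
; Tick also pins the gizmo to the target, world-aligned and scaled by player distance.
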(event EventTick
  (params (DeltaSeconds :type Float%20%28single-precision%29))
  (Utilities|FlowControl|Sequence
    (:then_0
      (CallFunction|FRotateTarget))
    (:then_1
      (CallFunction|FGizmoSize))))

(event EventBeginPlay
  (bind _asplayer_desktop (Utilities|Casting|CastToPlayer_Desktop (Game|GetPlayerCharacter 0)))
  (Variables|Referances|SetREF_Player _asplayer_desktop)
  (bind _asgizmo_base (Utilities|Casting|CastToGizmoBase (Actor|GetParentActor)))
  (Variables|Referances|SetREF_Gizmo_Base _asgizmo_base)
  (Input|EnableInput (Game|GetPlayerController 0))
  (Variables|/Script/Engine.PlayerController|SetbEnableClickEvents (Game|GetPlayerController 0) true))

(event OnClicked(Y_Mesh)
  (params (TouchedComponent :type Primitive%20Component%20Object%20Reference) (ButtonPressed :type Key%20Structure :default "None"))
  (Variables|Default|SetSelected_Axis (Utilities|Array|Get(acopy) (Variables|/Script/Engine.ActorComponent|GetComponentTags TouchedComponent))))

(event OnClicked(Z_Mesh)
  (params (TouchedComponent :type Primitive%20Component%20Object%20Reference) (ButtonPressed :type Key%20Structure :default "None"))
  (Variables|Default|SetSelected_Axis (Utilities|Array|Get(acopy) (Variables|/Script/Engine.ActorComponent|GetComponentTags TouchedComponent))))

(event OnClicked(X_Mesh)
  (params (TouchedComponent :type Primitive%20Component%20Object%20Reference) (ButtonPressed :type Key%20Structure :default "None"))
  (Variables|Default|SetSelected_Axis (Utilities|Array|Get(acopy) (Variables|/Script/Engine.ActorComponent|GetComponentTags TouchedComponent))))

(fn ConstructionScript)

(fn FRotateTarget
  (Utilities|IsValid (Variables|Referances|GetREF_Player)
    (:Is%20Valid
      (Utilities|IsValid (Variables|/Script/GizmoSystem.GizmoBase|GetGizmoTarget (Variables|Referances|GetREF_Gizmo_Base))
        (:Is%20Valid
          (if (not (Utilities|ForbiddenKeys))
            (if (Utilities|DetectMovement)
              (if (> (Math|Vector|DotProduct (Math|Vector|GetForwardVector (Variables|/Game/Player/Desktop/Player_Desktop.Player_Desktop_C|GetVRCamera (Variables|Referances|GetREF_Player))) (Math|Vector|Normalize (- (Transformation|GetWorldLocation (Variables|/Script/GizmoSystem.GizmoBase|GetGizmoTarget (Variables|Referances|GetREF_Gizmo_Base))) (Transformation|GetWorldLocation (Variables|/Game/Player/Desktop/Player_Desktop.Player_Desktop_C|GetVRCamera (Variables|Referances|GetREF_Player)))))) 0.5)
                (switch name (Variables|Default|GetSelected_Axis)
                  (:X_Mesh
                    (CallFunction|FRotateX))
                  (:Y_Mesh
                    (CallFunction|FRotateY))
                  (:Z_Mesh
                    (CallFunction|FRotateZ)))
                (return)))))))))

(fn FGizmoSize
  (bind _defaultsceneroot (Variables|Default|GetDefaultSceneRoot))
  (bind _ref_player (Variables|Referances|GetREF_Player))
  (bind _returnvalue (Transformation|GetWorldLocation _defaultsceneroot))
  (bind _capsulecomponent (Variables|/Script/Engine.Character|GetCapsuleComponent _ref_player))
  (bind _returnvalue_2 (Transformation|GetWorldLocation _capsulecomponent))
  (bind _returnvalue_3 (Math|Vector|Distance(Vector) _returnvalue_2 _returnvalue))
  (bind _returnvalue_4 (/ _returnvalue_3 7.5e+02))
  (Transformation|SetWorldTransform (Variables|Default|GetDefaultSceneRoot) (Math|Transform|MakeTransform (.location (Transformation|GetWorldTransform (Variables|/Script/GizmoSystem.GizmoBase|GetGizmoTarget (Variables|Referances|GetREF_Gizmo_Base)))) "0, 0, 0" (Math|Vector|MakeVector _returnvalue_4 _returnvalue_4 _returnvalue_4)) false false)
  (Transformation|SetWorldRotation (Variables|Default|GetDefaultSceneRoot) "0, 0, 0" false false)
  (return))

(fn FRotateY
  (bind _returnvalue (Game|GetPlayerController 0))
  (bind (_deltax _deltay) (Class|PlayerController|GetInputMouseDelta _returnvalue))
  (LocalVariables|SetAxis_Forward (Math|Vector|GetRightVector (Variables|Default|GetY_Mesh)))
  (LocalVariables|SetNormal_Vector (Utilities|HorizontalNormal (Variables|Default|GetY_Mesh)))
  (Transformation|AddWorldRotation (Variables|/Script/GizmoSystem.GizmoBase|GetGizmoTarget (Variables|Referances|GetREF_Gizmo_Base)) (Math|Rotator|MakeRotator 0.0 (Math|Float|Lerp (* _deltay (select (>= (Math|Float|Absolute(Float) (.z (LocalVariables|GetAxis_Forward))) 0.75) (select (>= (.z (LocalVariables|GetAxis_Forward)) 0.0) -5.0 5.0) (select (> (Math|Vector|DotProduct (LocalVariables|GetAxis_Forward) (LocalVariables|GetNormal_Vector)) 0.0) -5.0 5.0))) (* (select (> (.z (Math|Vector|CrossProduct (LocalVariables|GetAxis_Forward) (LocalVariables|GetNormal_Vector))) 0.0) 5.0 -5.0) _deltax) (Math|Float|Clamp(Float) (Math|Float|Absolute(Float) (.z (Math|Vector|CrossProduct (LocalVariables|GetAxis_Forward) (LocalVariables|GetNormal_Vector)))))) 0.0) false false)
  (return))

(fn FRotateX
  (bind _returnvalue (Game|GetPlayerController 0))
  (bind (_deltax _deltay) (Class|PlayerController|GetInputMouseDelta _returnvalue))
  (LocalVariables|SetAxis_Forward (Math|Vector|GetRightVector (Variables|Default|GetX_Mesh)))
  (LocalVariables|SetNormal_Vector (Utilities|HorizontalNormal (Variables|Default|GetX_Mesh)))
  (Transformation|AddWorldRotation (Variables|/Script/GizmoSystem.GizmoBase|GetGizmoTarget (Variables|Referances|GetREF_Gizmo_Base)) (Math|Rotator|MakeRotator (Math|Float|Lerp (* _deltay (select (>= (Math|Float|Absolute(Float) (.z (LocalVariables|GetAxis_Forward))) 0.75) (select (>= (.z (LocalVariables|GetAxis_Forward)) 0.0) 5.0 -5.0) (select (> (Math|Vector|DotProduct (LocalVariables|GetAxis_Forward) (LocalVariables|GetNormal_Vector)) 0.0) -5.0 5.0))) (* (select (> (.z (Math|Vector|CrossProduct (LocalVariables|GetAxis_Forward) (LocalVariables|GetNormal_Vector))) 0.0) 5.0 -5.0) _deltax) (Math|Float|Clamp(Float) (Math|Float|Absolute(Float) (.z (Math|Vector|CrossProduct (LocalVariables|GetAxis_Forward) (LocalVariables|GetNormal_Vector)))))) 0.0 0.0) false false)
  (return))

(fn FRotateZ
  (Transformation|AddWorldRotation (Variables|/Script/GizmoSystem.GizmoBase|GetGizmoTarget (Variables|Referances|GetREF_Gizmo_Base)) (Math|Rotator|MakeRotator 0.0 0.0 (* -5.0 (.DeltaX (Class|PlayerController|GetInputMouseDelta (Game|GetPlayerController 0))))) false false)
  (return))